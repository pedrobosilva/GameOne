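; Generic base character, apparently for enemies, that turns its mesh to face the player and walks toward them.
; BeginPlay caches friction and max health, applies walk speed, and binds itself to its health bar widget.
; Tick yaws the mesh at player 0 with a -90° model offset and feeds movement input along the corrected forward vector.
; Input mapping, move and dodge logic are present but disconnected, leaving those input events empty.
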(event EventBeginPlay
  (CallFunction|Start))

(event Collision|EventActorBeginOverlap
  (params (OtherActor :type Actor%20Object%20Reference)))

(event EventTick
  (params (DeltaSeconds :type Float%20%28single-precision%29))
  (CallFunction|LooktoPlayer)
  (CallFunction|MovementForward))

(event Custom|Start
  (CallFunction|SetVariables)
  (CallFunction|SetWidgets))

(event Input|EnhancedActionEvents|EnhancedInputActionIA_Dodge
  (params (ActionValue :type Boolean) (ElapsedSeconds :type Float%20%28double-precision%29) (TriggeredSeconds :type Float%20%28double-precision%29) (InputAction :type Input%20Action%20Object%20Reference :default "/Game/Input/Gameplay/Actions/IA_Dodge.IA_Dodge")))

(event Custom|ChangeState_to_Dodge)

(event Custom|SetVariables
  (Variables|Default|SetNormalFriction (Variables|/Script/Engine.CharacterMovementComponent|GetGroundFriction (Variables|Character|GetCharacterMovement)))
  (Variables|Default|SetmaxHealth (Variables|Default|GetcurrentHealth))
  (Variables|/Script/Engine.CharacterMovementComponent|SetMaxWalkSpeed (Variables|Character|GetCharacterMovement) (Variables|Default|GetMovementSpeed)))

(event Custom|Movement%20Handler
  (if (Utilities|Operators|EqualEqual :A (Math|Vector|VectorGetAbs (Variables|/Script/Engine.MovementComponent|GetVelocity (Variables|Character|GetCharacterMovement))))
    (Utilities|FlowControl|Delay 1.0)
    (Variables|Default|SetCurrentPlayerState "NewEnumerator0")))

(event Input|EnhancedActionEvents|EnhancedInputActionIA_Move
  (params (ActionValue :type Vector%202D%20Structure) (ElapsedSeconds :type Float%20%28double-precision%29) (TriggeredSeconds :type Float%20%28double-precision%29) (InputAction :type Input%20Action%20Object%20Reference :default "/Game/Input/Gameplay/Actions/IA_Move.IA_Move")))

(event Custom|SetWidgets
  (bind _aswb_generic_health_bar (Utilities|Casting|CastToWB_GenericHealth_Bar (UserInterface|GetWidget (Variables|Default|GetWidget))))
  (Variables|/Game/Widgets/WB_GenericHealth_Bar.WB_GenericHealth_Bar_C|SetGenericCharacter _aswb_generic_health_bar self))

(event Custom|Movement_Forward
  (Pawn|Input|AddMovementInput (Math|Vector|RotateVector (Math|Vector|GetForwardVector (Variables|Character|GetMesh)) "0.000000,90.000000,0.000000") 1.0 false))

(event Custom|LookToPlayer
  (Transformation|SetWorldRotation (Variables|Character|GetMesh) (Math|Rotator|MakeRotator 0.0 0.0 (.yaw (Math|Rotator|FindLookatRotation (Transformation|GetWorldLocation (Variables|Character|GetMesh)) (Transformation|GetActorLocation (Game|GetPlayerCharacter 0))))) false false)
  (Transformation|AddRelativeRotation (Variables|Character|GetMesh) "0.000000,-90.000000,0.000000" false false))

(fn ConstructionScript)

(fn GetModelForwardVector
  (params (Mesh :type Scene%20Component%20Object%20Reference))
  (return (Math|Vector|RotateVector (Math|Vector|GetForwardVector Mesh) "0.000000,90.000000,0.000000")))