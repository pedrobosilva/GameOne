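; BP_Generic_Spawner is a generic spawner actor that creates a passed-in class and can be rotated on demand.
; SpawnBlueprint spawns the class at the root's world transform and casts it to BP_Forward_Projectile, with the Arrow-based repositioning left disconnected.
; RotateSpawner sets yaw clockwise or counter-clockwise using delta time, but multiplies the whole summed yaw by speed, not just the step.
; Neither event is called within this Blueprint.
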(event EventBeginPlay)

(event Collision|EventActorBeginOverlap
  (params (OtherActor :type Actor%20Object%20Reference)))

(event EventTick
  (params (DeltaSeconds :type Float%20%28single-precision%29)))

(event Custom|SpawnBlueprint
  (params (ObjectToSpawn :type Actor%20Class%20Reference))
  (bind _returnvalue (Game|SpawnActorfromClass ObjectToSpawn (Transformation|GetWorldTransform (Variables|Default|GetDefaultSceneRoot)) "Undefined" "MultiplyWithRoot" 0 0))
  (Utilities|Casting|CastToBP_Forward_Projectile _returnvalue))

(event Custom|RotateSpawner
  (params (CounterClock :type Boolean) (RotatioSpeed :type Float%20%28double-precision%29))
  (bind _returnvalue (Utilities|Time|GetWorldDeltaSeconds))
  (bind _self self)
  (bind _returnvalue_2 (Transformation|GetActorRotation _self))
  (if CounterClock
    (Transformation|SetActorRotation _self (Math|Rotator|MakeRotator 0.0 0.0 (* (+ (.yaw _returnvalue_2) _returnvalue) RotatioSpeed)))
    (else
      (Transformation|SetActorRotation _self (Math|Rotator|MakeRotator 0.0 0.0 (* (- (.yaw _returnvalue_2) _returnvalue) RotatioSpeed))))))

(fn ConstructionScript)