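; Projectile spawner actor that periodically emits BP_Forward_Projectile while rotating clockwise.
; Tick calls the parent tick, then uses a Delay of SpawnRate to throttle each cycle of spawning followed by a RotateSpawner step.
; Rotation therefore advances only when a projectile spawns, not every frame.
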(event EventBeginPlay
  (|CallParentFunction) ; This node is disabled and will not be called.\nDrag off pins to build functionality.
)

(event Collision|EventActorBeginOverlap
  (params (OtherActor :type Actor%20Object%20Reference))
  (|CallParentFunction OtherActor) ; This node is disabled and will not be called.\nDrag off pins to build functionality.
)

(event EventTick
  (params (DeltaSeconds :type Float%20%28single-precision%29))
  (|CallParentFunction DeltaSeconds)
  (Utilities|FlowControl|Delay (Variables|Default|GetSpawnRate))
  (CallFunction|SpawnBlueprint "/Game/Projectiles/BP_Forward_Projectile.BP_Forward_Projectile_C")
  (CallFunction|RotateSpawner false 2.0))

(fn ConstructionScript
  (|CallParentFunction))