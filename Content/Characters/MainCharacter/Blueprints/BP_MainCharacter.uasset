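; Player character Blueprint with Enhanced Input movement, a cooldown-limited dodge and a health bar widget linked on BeginPlay.
; Movement follows world X/Y axes and rotates the mesh toward velocity, compensating for a 90-degree yaw offset.
; Dodge launches along the model's forward vector and sets the Dodging state, which blocks movement until EndDodge, never called here, restores Idle or Moving.
; MovementHandler and ChangeState_to_Dodge are empty stubs.
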(event EventBeginPlay
  (CallFunction|Start))

(event Collision|EventActorBeginOverlap
  (params (OtherActor :type Actor%20Object%20Reference)))

(event EventTick
  (params (DeltaSeconds :type Float%20%28single-precision%29))
  (Utilities|FlowControl|Sequence
    (:then_0
      (if (Utilities|Enum|NotEqual(Enum) (Variables|Default|GetCurrentPlayerState) "NewEnumerator2")
        (CallFunction|MovementHandler)))))

(event Custom|Start
  (bind _asplayer_controller (Utilities|Casting|CastToPlayerController (Pawn|GetController)))
  (Utilities|IsValid (PlayerController|LocalPlayerSubsystems|GetEnhancedInputLocalPlayerSubsystem _asplayer_controller)
    (:Is%20Valid
      (Input|AddMappingContext (PlayerController|LocalPlayerSubsystems|GetEnhancedInputLocalPlayerSubsystem _asplayer_controller) "/Game/Input/Gameplay/IM_Gameplay.IM_Gameplay" 0 "(bIgnoreAllPressedKeysUntilRelease=True,bForceImmediately=False,bNotifyUserSettings=False)")
      (CallFunction|SetVariables)
      (CallFunction|SetWidgets))))

(event Custom|EndDodge
  (if (> (Math|Vector2D|Vector2DLength (Variables|Default|GetCurrentDesiredDirection)) 0.0)
    (Variables|Default|SetCurrentPlayerState "NewEnumerator1")
    (else
      (Variables|Default|SetCurrentPlayerState "NewEnumerator0"))))

(event Input|EnhancedActionEvents|EnhancedInputActionIA_Dodge
  (params (ActionValue :type Boolean) (ElapsedSeconds :type Float%20%28double-precision%29) (TriggeredSeconds :type Float%20%28double-precision%29) (InputAction :type Input%20Action%20Object%20Reference :default "/Game/Input/Gameplay/Actions/IA_Dodge.IA_Dodge"))
  (Development|PrintString (Utilities|String|ToString(Vector) (stale _modelforward)))
  (Utilities|FlowControl|DoOnce false :!label _label
    (:Completed
      (Utilities|FlowControl|Sequence
        (:then_0
          (Utilities|FlowControl|Delay (Variables|Default|GetDodgeCooldown))
          (goto _label Reset))
        (:then_1
          (bind _modelforward (CallFunction|GetModelForwardVector (Variables|Character|GetMesh)))
          (if (Utilities|Enum|NotEqual(Enum) (Variables|Default|GetCurrentPlayerState) "NewEnumerator2")
            (Variables|/Script/Engine.MovementComponent|SetVelocity (Variables|Character|GetCharacterMovement) "0, 0, 0")
            (Character|LaunchCharacter (* (Variables|Default|GetDodgeForce) _modelforward) false false)
            (Variables|/Script/Engine.CharacterMovementComponent|SetGroundFriction (Variables|Character|GetCharacterMovement) (Variables|Default|GetDodgeFriction))
            (Variables|Default|SetCurrentPlayerState "NewEnumerator2")
            (Variables|/Script/Engine.CharacterMovementComponent|SetGroundFriction (Variables|Character|GetCharacterMovement) (Variables|Default|GetNormalFriction))))))))

(event Custom|ChangeState_to_Dodge)

(event Custom|SetVariables
  (Variables|Default|SetNormalFriction (Variables|/Script/Engine.CharacterMovementComponent|GetGroundFriction (Variables|Character|GetCharacterMovement)))
  (Variables|Default|SetmaxHealth (Variables|Default|GetcurrentHealth)))

(event Custom|Movement%20Handler)

(event Input|EnhancedActionEvents|EnhancedInputActionIA_Move
  (params (ActionValue :type Vector%202D%20Structure) (ElapsedSeconds :type Float%20%28double-precision%29) (TriggeredSeconds :type Float%20%28double-precision%29) (InputAction :type Input%20Action%20Object%20Reference :default "/Game/Input/Gameplay/Actions/IA_Move.IA_Move"))
  (if (Utilities|Enum|NotEqual(Enum) (Variables|Default|GetCurrentPlayerState) "NewEnumerator2")
    (Variables|Default|SetCurrentDesiredDirection (Math|Vector2D|MakeVector2D (.x ActionValue) (.y ActionValue)))
    (switch Utilities|FlowControl|Switch|SwitchonENUM_PlayerState (Variables|Default|GetCurrentPlayerState)
      (:NewEnumerator0
        _)
      (:NewEnumerator1
        _))
    (Pawn|Input|AddMovementInput "1.000000,0.000000,0.000000" (.x ActionValue) false)
    (Pawn|Input|AddMovementInput "0.000000,1.000000,0.000000" (.y ActionValue) false)
    (Transformation|SetRelativeRotation (Variables|Character|GetMesh) (Math|Conversions|RotationFromXVector (Math|Vector|RotateVector (Variables|/Script/Engine.MovementComponent|GetVelocity (Variables|Character|GetCharacterMovement)) "0.000000,-90.000000,0.000000")) false false)
    (Variables|Default|SetCurrentPlayerState "NewEnumerator1")
    (else
      (Variables|Default|SetCurrentDesiredDirection ""))))

(event Custom|SetWidgets
  (bind _aswb_player_health_bar (Utilities|Casting|CastToWB_PlayerHealth_Bar (UserInterface|GetWidget (Variables|Default|GetWidget))))
  (Variables|/Game/Widgets/WB_PlayerHealth_Bar.WB_PlayerHealth_Bar_C|SetCharacterReference _aswb_player_health_bar self))

(fn ConstructionScript)

(fn GetModelForwardVector
  (params (Mesh :type Scene%20Component%20Object%20Reference))
  (return (Math|Vector|RotateVector (Math|Vector|GetForwardVector Mesh) "0.000000,90.000000,0.000000")))