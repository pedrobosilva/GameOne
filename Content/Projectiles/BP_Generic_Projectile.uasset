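; Generic projectile Blueprint offering callable movement behaviors (forward, start-stop, rotating, homing) and a lifespan setter, with no startup logic of its own.
; Forward movement sets ProjectileMovement speeds and, when accelerating, starts a looping timer that scales velocity multiplicatively.
; Start-stop reuses forward movement until a delay enables deceleration, which reduces only X velocity by delta time and prints debug values.
; Rotation adds yaw by delta time, while homing configures a supplied movement component's target and acceleration.
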(event EventBeginPlay)

(event Collision|EventActorBeginOverlap
  (params (OtherActor :type Actor%20Object%20Reference)))

(event EventTick
  (params (DeltaSeconds :type Float%20%28single-precision%29)))

(event Custom|Movement_Start_Stop
  (params (isAccelerating :type Boolean) (acceleration :type Float%20%28double-precision%29) (Max%20Speed :type Float%20%28double-precision%29) (Initial%20Speed :type Float%20%28double-precision%29) (TimeToDecelerate :type Float%20%28double-precision%29) (deceleration :type Float%20%28double-precision%29))
  (bind _projectilemovement (Variables|Default|GetProjectileMovement))
  (bind _projectilemovement_2 (Variables|Default|GetProjectileMovement))
  (Utilities|FlowControl|Sequence
    (:then_0
      (if (stale _output_get_2)
        (if (> (Math|Float|Absolute(Float) (Math|Vector|VectorLength (stale _output_get))) 0.2)
          (bind _output_get (Variables|/Script/Engine.MovementComponent|SetVelocity _projectilemovement_2 (Math|Vector|MakeVector (- (.x (Variables|/Script/Engine.MovementComponent|GetVelocity _projectilemovement)) (* (Utilities|Time|GetWorldDeltaSeconds) deceleration)) (.y (Variables|/Script/Engine.MovementComponent|GetVelocity _projectilemovement)) (.z (Variables|/Script/Engine.MovementComponent|GetVelocity _projectilemovement)))))
          (Development|PrintString (Utilities|String|ToString(Float) (Math|Float|Absolute(Float) (Math|Vector|VectorLength _output_get))))
          (else
            (Variables|/Script/Engine.MovementComponent|SetVelocity _projectilemovement_2 "0, 0, 0")))
        (else
          (CallFunction|MovementForward isAccelerating acceleration Max%20Speed Initial%20Speed))))
    (:then_1
      (Utilities|FlowControl|Delay TimeToDecelerate)
      (bind _output_get_2 (Variables|Default|SetisDecelerating true)))
    (:then_2
      (Development|PrintString (Utilities|String|ToString(Vector) (Variables|/Script/Engine.MovementComponent|GetVelocity _projectilemovement))))))

(event Custom|Movement_Forward
  (params (isAccelerating :type Boolean) (acceleration :type Float%20%28double-precision%29) (Max%20Speed :type Float%20%28double-precision%29) (Initial%20Speed :type Float%20%28double-precision%29))
  (bind _returnvalue (Transformation|GetActorForwardVector))
  (bind _projectilemovement (Variables|Default|GetProjectileMovement))
  (Variables|/Script/Engine.ProjectileMovementComponent|SetInitialSpeed _projectilemovement Initial%20Speed)
  (Variables|/Script/Engine.ProjectileMovementComponent|SetMaxSpeed _projectilemovement Max%20Speed)
  (if isAccelerating
    (Utilities|FlowControl|Sequence
      (:then_0
        (Utilities|FlowControl|DoOnce false
          (:Completed
            (Variables|/Script/Engine.MovementComponent|SetVelocity (Variables|Default|GetProjectileMovement) (* (Math|Vector|MakeVector (.x _returnvalue) (.y _returnvalue) (.z _returnvalue)) (Math|Vector|MakeVector Initial%20Speed 1.0 1.0))))))
      (:then_1
        (Utilities|Time|SetTimerbyEvent (delegate Custom|IncrementSpeedByTime) 0.1 true true)))))

(event Custom|Movement_Rotate
  (params (RotateSpeed :type Float%20%28double-precision%29))
  (bind _returnvalue (Transformation|GetActorRotation))
  (Transformation|SetActorRotation (Math|Rotator|MakeRotator (.roll _returnvalue) (.pitch _returnvalue) (+ (* RotateSpeed (Utilities|Time|GetWorldDeltaSeconds)) (.yaw _returnvalue)))))

(event Custom|IncrementSpeedByTime
  (bind _projectilemovement (Variables|Default|GetProjectileMovement))
  (Variables|/Script/Engine.MovementComponent|SetVelocity _projectilemovement (* (* (stale Custom|Movement_Forward acceleration) 0.1) (Variables|/Script/Engine.MovementComponent|GetVelocity _projectilemovement))))

(event Custom|SetVariables)

(event Custom|Movement_Homing
  (params (Target :type Scene%20Component%20Object%20Reference) (Projectile%20Movement%20Component :type Projectile%20Movement%20Component%20Object%20Reference) (HomingAcelleration :type Float%20%28double-precision%29))
  (Variables|/Script/Engine.ProjectileMovementComponent|SetbIsHomingProjectile Projectile%20Movement%20Component true)
  (Variables|/Script/Engine.ProjectileMovementComponent|SetHomingTargetComponent Projectile%20Movement%20Component Target)
  (Variables|/Script/Engine.ProjectileMovementComponent|SetHomingAccelerationMagnitude Projectile%20Movement%20Component HomingAcelleration))

(event Custom|UseLifeSpan
  (params (Self_Ref :type Actor%20Object%20Reference) (LifeSpan :type Float%20%28double-precision%29))
  (Actor|SetLifeSpan Self_Ref LifeSpan))

(fn ConstructionScript)

(fn DecrementbyTime
  (params (StartTime :type Float%20%28double-precision%29)))